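; Player controller for turn-based tile combat that turns mouse hover and clicks into unit moves, attacks, pawn switches and turn endings.
; ActivateUnit has the grid manager build pathfinding and range data, which clicks read to act on empty, player or enemy tiles.
; Out-of-range enemies trigger move-then-attack through the unit's own movement logic, while EndUnitTurn asks the game mode for the next pawn.
; Tick updates markers and previews paths or attack lines.
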(event `self.ReceiveBeginPlay`
  ;[0 0.9833 1] Setup Blueprint Communication
  (bind _outactors (`GameplayStatics.GetAllActorsOfClass` (`self.Grid_Manager_Class_Ref`)))
  (set `self.Grid_Manager_Ref` (`KismetArrayLibrary.Array_Get` _outactors))
  (bind _outactors_2 (`GameplayStatics.GetAllActorsOfClass` (`self.GameModeClass_Ref`)))
  (set `self.GameMode_Ref` (`KismetArrayLibrary.Array_Get` _outactors_2)))

(event `Activate Unit`
  (params (Unit :type "/Game/Blueprints/Pawns/Unit_Parent Object Reference"))
  (bind _grid_manager_ref (`self.Grid_Manager_Ref`))
  (bind _index (`/Game/Blueprints/Pawns/Unit_Parent.Index` Unit))
  (bind _current_move (`/Game/Blueprints/Pawns/Unit_Parent.Current Move` Unit))
  (bind _range (`/Game/Blueprints/Pawns/Unit_Parent.Range` Unit))
  (bind _grid_manager_ref_2 (`self.Grid_Manager_Ref`))
  ;[0 1 0.003575] Begin Unit Turn
  (set `self.DisableInput_0` false)
  (set `/Game/Blueprints/Pawns/Unit_Parent.Idle` true Unit)
  (`/Game/Blueprints/Gameplay/BP_Grid_Manager.Pathfinding` (`self.Grid_Manager_Ref`) _index _current_move 0 (`/Game/Blueprints/Pawns/Unit_Parent.Diagonal Movement` Unit) (`/Game/Blueprints/Pawns/Unit_Parent.Cross Corners` Unit) false false)
  (`/Game/Blueprints/Gameplay/BP_Grid_Manager.Find Tiles In Range` (`self.Grid_Manager_Ref`) _index _range true (> _current_move 0) "NewEnumerator1" true false (* _range (/ (+ (`/Game/Blueprints/Gameplay/BP_Grid_Manager.TileBoundsX` _grid_manager_ref_2) (`/Game/Blueprints/Gameplay/BP_Grid_Manager.TileBoundsY` _grid_manager_ref_2)) 2.0)) 1)
  (`/Game/Blueprints/Gameplay/BP_Grid_Manager.Set Marker Visibility` _grid_manager_ref true (`/Game/Blueprints/Gameplay/BP_Grid_Manager.Hover Marker Decal` _grid_manager_ref) (`/Game/Blueprints/Gameplay/BP_Grid_Manager.HoverMarker` _grid_manager_ref)))

(event `InputAction|Click`
  (params (Key :type "Key Structure" :default "AnyKey"))
  (bind _targetispawn (`self.TargetIsPawn`))
  (bind _grid_manager_ref (`self.Grid_Manager_Ref`))
  (bind _grid_manager_ref_2 (`self.Grid_Manager_Ref`))
  (bind _grid_manager_ref_3 (`self.Grid_Manager_Ref`))
  (bind _grid_manager_ref_4 (`self.Grid_Manager_Ref`))
  (bind (_closest_index _index_found) (`/Game/Blueprints/Gameplay/BP_Grid_Manager.Reachable index closest to target` (`self.Grid_Manager_Ref`)))
  (bind _currentpawn (`/Game/Blueprints/Gameplay/ATBTT_GameMode.CurrentPawn` (`self.GameMode_Ref`)))
  (bind _currentpawn_2 (`/Game/Blueprints/Gameplay/ATBTT_GameMode.CurrentPawn` (`self.GameMode_Ref`)))
  (bind _currentpawn_3 (`/Game/Blueprints/Gameplay/ATBTT_GameMode.CurrentPawn` (`self.GameMode_Ref`)))
  (bind _targetmarker (`/Game/Blueprints/Gameplay/BP_Grid_Manager.TargetMarker` _grid_manager_ref_3))
  (bind _target_marker_decal (`/Game/Blueprints/Gameplay/BP_Grid_Manager.Target Marker Decal` _grid_manager_ref_3))
  (bind _currentpawn_4 (`/Game/Blueprints/Gameplay/ATBTT_GameMode.CurrentPawn` (`self.GameMode_Ref`)))
  (bind (_item_index _item_cost) (break `/Game/Blueprints/Gameplay/Structs/Struct_Pathfinding` (`KismetArrayLibrary.Array_Get` (`/Game/Blueprints/Gameplay/BP_Grid_Manager.CanMoveToArray` (`self.Grid_Manager_Ref`)) (`self.Target Index`))))
  (bind (_item_index_2 _item_cost_2) (break `/Game/Blueprints/Gameplay/Structs/Struct_Pathfinding` (`KismetArrayLibrary.Array_Get` (`/Game/Blueprints/Gameplay/BP_Grid_Manager.CanMoveToArray` (`self.Grid_Manager_Ref`)) (`self.ClickedTile`))))
  (bind (_item_index_3 _item_cost_3) (break `/Game/Blueprints/Gameplay/Structs/Struct_Pathfinding` (`KismetArrayLibrary.Array_Get` (`/Game/Blueprints/Gameplay/BP_Grid_Manager.CanMoveToArray` (`self.Grid_Manager_Ref`)) (`self.ClickedTile`))))
  (bind _item (`KismetArrayLibrary.Array_Get` (`/Game/Blueprints/Gameplay/BP_Grid_Manager.PawnActorArray` (`self.Grid_Manager_Ref`)) (`self.ClickedTile`)))
  (bind _index (`/Game/Blueprints/Pawns/Unit_Parent.Index` (`/Game/Blueprints/Gameplay/ATBTT_GameMode.CurrentPawn` (`self.GameMode_Ref`))))
  (bind _returnvalue (> _item_cost_3 0))
  ;[1 0.7618 0] Choose action depending on tile clicked
  (:`Pressed`
    (if (`/Game/Blueprints/Gameplay/ATBTT_GameMode.PlayerTurn` (`self.GameMode_Ref`))
      (if (not (`self.DisableInput_0`))
        (bind (_index_2 _location _tracehit) (`/Game/Blueprints/Gameplay/BP_Grid_Manager.Get hit tile location and index` (`self.Grid_Manager_Ref`)))
        (if _tracehit
          (set `self.ClickedTile` _index_2)
          (switch `/Game/Blueprints/Gameplay/Enums/Enum_Faction` (`KismetArrayLibrary.Array_Get` (`/Game/Blueprints/Gameplay/BP_Grid_Manager.PawnArray` (`self.Grid_Manager_Ref`)) _index_2) ; What pawn is on the clicked tile?
            (:`NewEnumerator3`
              ;[0 0.325 0.06358] Initiate movement towards and/or attacking target
              (set `self.TargetIsPawn` false)
              (if (and _returnvalue (<= _item_cost_3 (`/Game/Blueprints/Pawns/Unit_Parent.Current Move` (`/Game/Blueprints/Gameplay/ATBTT_GameMode.CurrentPawn` (`self.GameMode_Ref`))))) :!label _label
                (set `self.DisableInput_0` true :!label _label_2)
                (`/Game/Blueprints/Gameplay/BP_Grid_Manager.Set Marker Location` (`self.Grid_Manager_Ref`) (0.0 0.0 0.0) true (`self.ClickedTile`) _target_marker_decal _targetmarker)
                (`/Game/Blueprints/Gameplay/BP_Grid_Manager.Set Marker Location` _grid_manager_ref_3 (0.0 0.0 0.0) true (`self.ClickedTile`) _target_marker_decal _targetmarker) ; Set target marker to the target tile
                (`/Game/Blueprints/Gameplay/BP_Grid_Manager.Set Marker Visibility` (`self.Grid_Manager_Ref`) true _target_marker_decal _targetmarker)
                (if (`self.TargetIsPawn`)
                  (if (not (== _item_cost_2 0))
                    (set `self.Target Index` (`KismetArrayLibrary.Array_Get` (`/Game/Blueprints/Gameplay/BP_Grid_Manager.Path Index Array` (`self.Grid_Manager_Ref`)) 1)) ; Set the end of the path to the tile in front of the enemy
                    (`/Game/Blueprints/Gameplay/BP_Grid_Manager.Find path within pathfinding array` (`self.Grid_Manager_Ref`) (`self.ClickedTile`) true false false :!label _label_3)
                    (set `/Game/Blueprints/Pawns/Unit_Parent.HasActedThisTurn` true (`/Game/Blueprints/Gameplay/ATBTT_GameMode.CurrentPawn` (`self.GameMode_Ref`)))
                    (`/Game/Blueprints/Gameplay/BP_Grid_Manager.Clear all in range mesh markers` _grid_manager_ref_2)
                    (`/Game/Blueprints/Gameplay/BP_Grid_Manager.Destroy and clear spline path` _grid_manager_ref_2)
                    (`KismetArrayLibrary.Array_Set` (`/Game/Blueprints/Gameplay/BP_Grid_Manager.PawnArray` (`self.Grid_Manager_Ref`)) _index "NewEnumerator3")
                    (`KismetArrayLibrary.Array_Set` (`/Game/Blueprints/Gameplay/BP_Grid_Manager.PawnActorArray` (`self.Grid_Manager_Ref`)) _index null)
                    (`/Game/Blueprints/Pawns/Unit_Parent.Begin Movement` (`/Game/Blueprints/Gameplay/ATBTT_GameMode.CurrentPawn` (`self.GameMode_Ref`)) (`KismetMathLibrary.Conv_BoolToInt` _targetispawn) _targetispawn) ; Begin pawn movement (continued in event graph Unit_Parent)
                    (`/Game/Blueprints/Gameplay/BP_Grid_Manager.Set Marker Visibility` _grid_manager_ref_4 false (`/Game/Blueprints/Gameplay/BP_Grid_Manager.Hover Marker Decal` _grid_manager_ref_4) (`/Game/Blueprints/Gameplay/BP_Grid_Manager.HoverMarker` _grid_manager_ref_4))
                    (if (`/Game/Blueprints/Pawns/Unit_Parent.Can Split Up Move` (`/Game/Blueprints/Gameplay/ATBTT_GameMode.CurrentPawn` (`self.GameMode_Ref`)))
                      (set `/Game/Blueprints/Pawns/Unit_Parent.Current Move` (- (`/Game/Blueprints/Pawns/Unit_Parent.Current Move` _currentpawn) _item_cost) _currentpawn)
                      (else
                        (set `/Game/Blueprints/Pawns/Unit_Parent.Current Move` 0 _currentpawn)))
                    (`KismetArrayLibrary.Array_Clear` (`/Game/Blueprints/Gameplay/BP_Grid_Manager.CanMoveToArray` (`self.Grid_Manager_Ref`))))
                  (else
                    (set `self.Target Index` (`self.ClickedTile`))
                    (goto _label_3)))
                (else
                  (if _returnvalue
                    (set `self.TargetIsPawn` false)
                    (if _index_found
                      (set `self.ClickedTile` _closest_index)
                      (goto _label_2)
                      (else
                        _))
                    (else
                      (set `self.TargetIsPawn` false)))
                  (set `self.DisableInput_0` false)
                  (if (== (`/Game/Blueprints/Pawns/Unit_Parent.Current Move` (`/Game/Blueprints/Gameplay/ATBTT_GameMode.CurrentPawn` (`self.GameMode_Ref`))) 0)
                    (`self.End Unit Turn` 0.0)))))
            (:`NewEnumerator0`
              ;[1 0.9168 0] End turn if the current unit is clicked
              (if (== (`/Game/Blueprints/Pawns/Unit_Parent.Index` (`/Game/Blueprints/Gameplay/ATBTT_GameMode.CurrentPawn` (`self.GameMode_Ref`))) (`self.ClickedTile`))
                (if (> (`/Game/Blueprints/Pawns/Unit_Parent.Current Move` (`/Game/Blueprints/Gameplay/ATBTT_GameMode.CurrentPawn` (`self.GameMode_Ref`))) 0)
                  (set `/Game/Blueprints/Pawns/Unit_Parent.Current Move` 0 _currentpawn_4)
                  (`self.Activate Unit` _currentpawn_4)
                  (else
                    (`self.End Unit Turn` 0.0)))
                (elif (`/Game/Blueprints/Gameplay/BP_Grid_Manager.Can Player Switch Pawns?` (`self.Grid_Manager_Ref`))
                  ;[1 1 1] If CanPlayerSwitchPawns is true and a pawn that has not acted is click, switch to this pawn
                  (if (not (`/Game/Blueprints/Pawns/Unit_Parent.HasActedThisTurn` _item))
                    (if (`/Game/Blueprints/Pawns/Unit_Parent.HasActedThisTurn` (`/Game/Blueprints/Gameplay/ATBTT_GameMode.CurrentPawn` (`self.GameMode_Ref`)))
                      (`/Game/Blueprints/Gameplay/ATBTT_GameMode.Let the First Pawn in Initiative Become the Last` (`self.GameMode_Ref`))
                      (set `/Game/Blueprints/Pawns/Unit_Parent.Current Move` (`/Game/Blueprints/Pawns/Unit_Parent.Max Move` _currentpawn_2) _currentpawn_2))
                    (`/Game/Blueprints/Gameplay/ATBTT_GameMode.Set Unit to First in Initiative` (`self.GameMode_Ref`) _item)
                    (`/Game/Blueprints/Gameplay/BP_Grid_Manager.Clear all in range mesh markers` (`self.Grid_Manager_Ref`))
                    (bind _output_get (set `/Game/Blueprints/Gameplay/ATBTT_GameMode.CurrentPawn` _item (`self.GameMode_Ref`)))
                    (`self.Activate Unit` _output_get)
                    (set `/Game/Blueprints/Gameplay/BP_Grid_Camera.IsPanning` false (`/Game/Blueprints/Gameplay/ATBTT_GameMode.BP_Grid_Camera_Ref` (`self.GameMode_Ref`)))))))
            (:`NewEnumerator1`
              ;[1 0.003995 0] Attack clicked target if within reach, or move towards it if it is not
              (if (> (`KismetArrayLibrary.Array_Get` (`/Game/Blueprints/Gameplay/BP_Grid_Manager.RangeArray` (`self.Grid_Manager_Ref`)) (`self.ClickedTile`)) 0)
                (set `self.DisableInput_0` true)
                (`/Game/Blueprints/Gameplay/BP_Grid_Manager.Clear all in range mesh markers` _grid_manager_ref)
                (`/Game/Blueprints/Gameplay/BP_Grid_Manager.Destroy and clear spline path` _grid_manager_ref)
                (`/Game/Blueprints/Pawns/Unit_Parent.Attack Victim` _currentpawn_3 (`KismetArrayLibrary.Array_Get` (`/Game/Blueprints/Gameplay/BP_Grid_Manager.PawnActorArray` (`self.Grid_Manager_Ref`)) (`self.ClickedTile`)))
                (set `/Game/Blueprints/Pawns/Unit_Parent.Idle` false _currentpawn_3)
                (else
                  (set `self.TargetIsPawn` true) ; If target is pawn is true the current unit will try to move to the tile next to the target and automatically attack
                  (goto _label))))))))))

(event `End Unit Turn`
  (params (Delay :type "Float (double-precision)" :default 0.0))
  ;[1 0 0.05054] End Unit Turn
  (`/Game/Blueprints/Gameplay/BP_Grid_Manager.Clear all in range mesh markers` (`self.Grid_Manager_Ref`))
  (`KismetSystemLibrary.Delay` Delay)
  (`/Game/Blueprints/Gameplay/ATBTT_GameMode.ChooseNextPawn` (`self.GameMode_Ref`) 0.0))

(event `self.ReceiveTick`
  (params (DeltaSeconds :type "Float (single-precision)"))
  (bind _grid_manager_ref (`self.Grid_Manager_Ref`))
  (bind _grid_manager_ref_2 (`self.Grid_Manager_Ref`))
  (bind _grid_manager_ref_3 (`self.Grid_Manager_Ref`))
  (bind _visibilitytraceheight (`/Game/Blueprints/Gameplay/BP_Grid_Manager.VisibilityTraceHeight` _grid_manager_ref_2))
  (bind (_item_index _item_cost) (break `/Game/Blueprints/Gameplay/Structs/Struct_Pathfinding` (`KismetArrayLibrary.Array_Get` (`/Game/Blueprints/Gameplay/BP_Grid_Manager.CanMoveToArray` (`self.Grid_Manager_Ref`)) (`self.CurrentTileHover`))))
  ;[0 0.003818 0.04] Display path on hover
  (`/Game/Blueprints/Gameplay/BP_Grid_Manager.Set Marker Location` _grid_manager_ref (`self.K2_GetActorLocation` (`/Game/Blueprints/Gameplay/ATBTT_GameMode.CurrentPawn` (`self.GameMode_Ref`))) false 0 (`/Game/Blueprints/Gameplay/BP_Grid_Manager.CurrentMarkerDecal` _grid_manager_ref) (`/Game/Blueprints/Gameplay/BP_Grid_Manager.CurrentPawnMarker` _grid_manager_ref)) ; Always set the position of the current marker to the current pawn
  (bind (_index _location _tracehit) (`/Game/Blueprints/Gameplay/BP_Grid_Manager.Get hit tile location and index` (`self.Grid_Manager_Ref`)))
  (if _tracehit
    (if (!= _index (`self.CurrentTileHover`))
      (set `self.CurrentTileHover` _index)
      (`/Game/Blueprints/Gameplay/BP_Grid_Manager.Set Marker Location` (`self.Grid_Manager_Ref`) (0.0 0.0 0.0) true (`self.CurrentTileHover`) (`/Game/Blueprints/Gameplay/BP_Grid_Manager.Hover Marker Decal` _grid_manager_ref_3) (`/Game/Blueprints/Gameplay/BP_Grid_Manager.HoverMarker` _grid_manager_ref_3))
      (`/Game/Blueprints/Gameplay/BP_Grid_Manager.Set Marker Location` _grid_manager_ref_3 (0.0 0.0 0.0) true (`self.CurrentTileHover`) (`/Game/Blueprints/Gameplay/BP_Grid_Manager.Hover Marker Decal` _grid_manager_ref_3) (`/Game/Blueprints/Gameplay/BP_Grid_Manager.HoverMarker` _grid_manager_ref_3)) ; Change the position ov the hover marker if the mouse is over a new grid tile
      (if (`/Game/Blueprints/Gameplay/ATBTT_GameMode.PlayerTurn` (`self.GameMode_Ref`))
        (if (`/Game/Blueprints/Pawns/Unit_Parent.Idle` (`/Game/Blueprints/Gameplay/ATBTT_GameMode.CurrentPawn` (`self.GameMode_Ref`)))
          (switch `/Game/Blueprints/Gameplay/Enums/Enum_Faction` (`KismetArrayLibrary.Array_Get` (`/Game/Blueprints/Gameplay/BP_Grid_Manager.PawnArray` (`self.Grid_Manager_Ref`)) (`self.CurrentTileHover`))
            (:`NewEnumerator3`
              (if (> _item_cost 0)
                (`/Game/Blueprints/Gameplay/BP_Grid_Manager.Find path within pathfinding array` (`self.Grid_Manager_Ref`) (`self.CurrentTileHover`) true true (`/Game/Blueprints/Gameplay/BP_Grid_Manager.DisplayPathAsSpline` (`self.Grid_Manager_Ref`)) :!label _label_4) ; Find and show a path from the path hovered to the tile the pathfinding array was generated from (generally the current pawn)
                (else
                  (if (`/Game/Blueprints/Gameplay/BP_Grid_Manager.DisplayPathAsSpline` (`self.Grid_Manager_Ref`)) :!label _label_5
                    (`/Game/Blueprints/Gameplay/BP_Grid_Manager.Destroy and clear spline path` (`self.Grid_Manager_Ref`))
                    (else
                      (`InstancedStaticMeshComponent.ClearInstances` (`/Game/Blueprints/Gameplay/BP_Grid_Manager.Path` (`self.Grid_Manager_Ref`))) ; Delete the old path markers (do nothing if path is displayed as path)
                    )))))
            (:`NewEnumerator0`
              (goto _label_5))
            (:`NewEnumerator1`
              (if (> (`KismetArrayLibrary.Array_Get` (`/Game/Blueprints/Gameplay/BP_Grid_Manager.RangeArray` (`self.Grid_Manager_Ref`)) (`self.CurrentTileHover`)) 1)
                (`/Game/Blueprints/Gameplay/BP_Grid_Manager.Display Straight Spline Between Points` _grid_manager_ref_2 (`self.CurrentTileHover`) _visibilitytraceheight (`/Game/Blueprints/Pawns/Unit_Parent.Index` (`/Game/Blueprints/Gameplay/ATBTT_GameMode.CurrentPawn` (`self.GameMode_Ref`))) _visibilitytraceheight) ; Display a straight line between pawns if a target within range is moused over
                (elif (> _item_cost 1)
                  (goto _label_4)
                  (else
                    (goto _label_5)))))))))
    (else
      (goto _label_5))))

(fn `UserConstructionScript`)